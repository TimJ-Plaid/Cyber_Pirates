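; Spawn volume actor for a tower defense prototype that spawns a limited run of AI actors at its Box component.
; BeginPlay opens a gate that Tick feeds every frame, with a Delay throttling spawns to roughly one per second.
; Each spawn increments a counter, and the StopSpawning event closes the gate once the count passes its hardcoded limit.
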(event EventStopSpawning
  (Utilities|FlowControl|Gate true) ; enters at Close
)

(event EventTick
  (params (DeltaSeconds :type Float%20%28single-precision%29))
  (Utilities|FlowControl|Gate true
    (:Exit
      (Utilities|FlowControl|Delay 1.0)
      (Game|SpawnActorfromClass "/Game/TowerDefPrototype/Blueprints/AI.AI_C" (Math|Conversions|ToTransform(Vector) (Transformation|GetWorldLocation (Variables|Default|GetBox))) "Undefined" 0 0)
      (Variables|Default|SetSpawnCount (+ (Variables|Default|GetSpawnCount) 1))
      (if (> (Variables|Default|GetSpawnCount) 15)
        (CallFunction|StopSpawning)))))

(event EventSpawnAI
  (Utilities|FlowControl|Gate true) ; enters at Open
)

(event EventBeginPlay
  (CallFunction|SpawnAI))

(fn ConstructionScript)