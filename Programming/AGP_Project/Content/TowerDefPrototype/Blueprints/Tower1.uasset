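; Tower defense turret prototype that detects AI actors in a collision volume, turns toward a target and fires bullets.
; Overlap begin records the AI and, without a current target, line-traces for one; overlap end clears it.
; A Tick-fed gate rotates the turret with RInterpTo, then a 0.2-second delay leads to spawning a bullet, or resetting if the AI is dead.
; AIArray collects entrants but is never read.
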(event OnComponentBeginOverlap(Detectioncollision)
  (params (OverlappedComponent :type Primitive%20Component%20Object%20Reference) (OtherActor :type Actor%20Object%20Reference) (OtherComp :type Primitive%20Component%20Object%20Reference) (OtherBodyIndex :type Integer) (bFromSweep :type Boolean) (SweepResult :type Hit%20Result%20Structure%20%28by%20ref%29))
  (bind _turret (Variables|Default|GetTurret))
  (bind _asai (Utilities|Casting|CastToAI OtherActor))
  (bind _output_get (Variables|Default|SetAiRef _asai))
  (Utilities|Array|Add (Variables|Default|GetAI_Array) _output_get)
  (if (Variables|Default|GetNOTargetSelected)
    (bind (_outhit _returnvalue) (Collision|LineTraceForObjects (Transformation|GetWorldLocation (Variables|Default|GetTurret)) (Transformation|GetWorldLocation (Variables|/Game/TowerDefPrototype/Blueprints/AI.AI_C|GetStaticMesh _asai)) (Utilities|Array|MakeArray "ObjectTypeQuery3") false 0 "ForDuration"))
    (bind _output_get_2 (Variables|Default|SettargetRef (.HitActor (Collision|BreakHitResult _outhit))))
    (if _returnvalue
      (Variables|Default|SetNOTargetSelected false)
      (Utilities|FlowControl|Gate true) ; enters at Open
      (else
        (Variables|Default|SetNOTargetSelected true)))
    (else
      (Utilities|FlowControl|Gate true) ; enters at Open
    )))

(event OnComponentEndOverlap(Detectioncollision)
  (params (OverlappedComponent :type Primitive%20Component%20Object%20Reference) (OtherActor :type Actor%20Object%20Reference) (OtherComp :type Primitive%20Component%20Object%20Reference) (OtherBodyIndex :type Integer))
  (bind _turret (Variables|Default|GetTurret))
  (Utilities|Casting|CastToAI OtherActor)
  (Variables|Default|SetNOTargetSelected true)
  (Utilities|FlowControl|Gate true) ; enters at Close
)

(event Custom|Shoot
  (Game|SpawnActorfromClass "/Game/TowerDefPrototype/Blueprints/Bbullet.Bbullet_C" (Math|Transform|MakeTransform (+ (Transformation|GetWorldLocation (Variables|Default|GetTurretHead)) "0.000000,20.000000,-10.000000") (Transformation|GetWorldRotation (Variables|Default|GetTurret)) "0.500000,0.500000,0.500000") "Undefined" 0 0))

(event Custom|Reset
  (bind _turret (Variables|Default|GetTurret))
  (Variables|Default|SetNOTargetSelected true)
  (Utilities|FlowControl|Gate true) ; enters at Toggle
)

(event EventBeginPlay)

(event Collision|EventActorBeginOverlap
  (params (OtherActor :type Actor%20Object%20Reference)))

(event EventTick
  (params (DeltaSeconds :type Float%20%28single-precision%29))
  (bind _turret (Variables|Default|GetTurret))
  (Utilities|FlowControl|Gate true
    (:Exit
      (Transformation|SetWorldRotation (Variables|Default|GetTurret) (Math|Interpolation|RInterpTo (Transformation|GetWorldRotation _turret) (Math|Rotator|FindLookatRotation (Transformation|GetWorldLocation _turret) (Transformation|GetActorLocation (stale OnComponentBeginOverlap(Detectioncollision) _output_get_2))) 1.0 (Variables|Default|GetTurretRotSpd)) false false)
      (Utilities|FlowControl|Delay 0.2)
      (if (Variables|/Game/TowerDefPrototype/Blueprints/AI.AI_C|GetIsDead (Variables|Default|GetAiRef))
        (CallFunction|Reset)
        (else
          (CallFunction|Shoot self))))))

(fn ConstructionScript)