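; Rail gun turret that automatically tracks and damages AI entering its line-of-sight sphere.
; Actor overlaps queue AI in an array, removing the first entry on exit, while Tick drives a gate opened on target lock.
; The gated path interpolates head rotation, then after a cooldown draws a debug trace and applies damage directly; the homing-bullet ShootFunction is unused.
; The construction script applies designer-set radius, meshes and materials.
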(event OnComponentBeginOverlap(RANGECUTOFF)
  (params (OverlappedComponent :type Primitive%20Component%20Object%20Reference) (OtherActor :type Actor%20Object%20Reference) (OtherComp :type Primitive%20Component%20Object%20Reference) (OtherBodyIndex :type Integer) (bFromSweep :type Boolean) (SweepResult :type Hit%20Result%20Structure%20%28by%20ref%29)))

(event OnComponentEndOverlap(RANGECUTOFF)
  (params (OverlappedComponent :type Primitive%20Component%20Object%20Reference) (OtherActor :type Actor%20Object%20Reference) (OtherComp :type Primitive%20Component%20Object%20Reference) (OtherBodyIndex :type Integer)))

(event Custom|TargetLocked
  ;[1 0.025 0.025] Check for every frame if Target is locked to follow target Rotation and Shoot
  (Utilities|FlowControl|Gate true) ; enters at Open
)

(event Custom|NoTarget
  ;[1 0.025 0.025] Check for every frame if Target is locked to follow target Rotation and Shoot
  (Utilities|FlowControl|Gate true) ; enters at Close
)

(event Collision|EventActorEndOverlap
  (params (OtherActor :type Actor%20Object%20Reference))
  ;[1 0.9363 0.009047] Remove Lock on Target upon exiting LINEOFSIGHT
  (Utilities|Casting|CastToAI OtherActor)
  (Utilities|Array|RemoveIndex (Variables|PrivateVariables|GetAIArrayRef))
  (if (== (Utilities|Array|Get(acopy) (Variables|PrivateVariables|GetAIArrayRef)) 0)
    (CallFunction|NoTarget)))

(event EventTick
  (params (DeltaSeconds :type Float%20%28single-precision%29))
  ;[1 0.025 0.025] Check for every frame if Target is locked to follow target Rotation and Shoot
  (Utilities|FlowControl|Sequence
    (:then_0
      (Utilities|FlowControl|Gate true
        (:Exit
          (Utilities|IsValid (Variables|PrivateVariables|GetTargetAI)
            (:Is%20Valid
              (CallFunction|TurretRotationonTargetAI)
              (Utilities|FlowControl|Delay (Variables|PublicVariables|GetCoolDownIntervalInDeltaSeconds))
              (Collision|LineTraceForObjects (Transformation|GetWorldLocation (Variables|Default|GetTurretBarrel)) (Transformation|GetActorLocation (Variables|PrivateVariables|GetTargetAI)) (Utilities|Array|MakeArray "ObjectTypeQuery3") false 0 "ForOneFrame")
              (Default|TakeDamage (Variables|PrivateVariables|GetTargetAI) (Variables|PublicVariables|GetTurretDamageValue)))))))
    (:then_1
      (if (Utilities|Array|ContainsItem (Variables|PrivateVariables|GetAIArrayRef) (Variables|PrivateVariables|GetAIRef))
        (Variables|PrivateVariables|SetTargetAI (Utilities|Array|Get(acopy) (Variables|PrivateVariables|GetAIArrayRef) (Variables|PrivateVariables|GetCurrentIndex)))
        (CallFunction|TargetLocked)))))

(event Collision|EventActorBeginOverlap
  (params (OtherActor :type Actor%20Object%20Reference))
  ;[1 0.9363 0.009047] Lock target on AI upon entering LINEOFSIGHT
  (bind _asai (Utilities|Casting|CastToAI OtherActor))
  (bind _output_get (Variables|PrivateVariables|SetAIRef _asai))
  (Utilities|Array|Add (Variables|PrivateVariables|GetAIArrayRef) _output_get))

(fn ConstructionScript
  ;[1 1 1] Designer editable Valures
  ;;[1 0.03 0.03] Line of Sight
  (Components|Sphere|SetSphereRadius (Variables|Default|Get%20LINEOFSIGHT) (Variables|PublicVariables|GetLineOfSight) true)
  ;;[0.01179 0.08912 1] StaticMesh
  (Components|StaticMesh|SetStaticMesh (Variables|Default|GetTurretBase) (Variables|PublicVariables|GetSM_TurretBase))
  (Components|StaticMesh|SetStaticMesh (Variables|Default|GetTurretHead) (Variables|PublicVariables|GetSM_TurretHead))
  (Components|StaticMesh|SetStaticMesh (Variables|Default|GetTurretBarrel) (Variables|PublicVariables|GetSM_TurretBarrel))
  ;;[0 1 0.1964] MaterialTexture
  (Rendering|Material|SetMaterial (Variables|Default|GetTurretBase) 0 (Variables|PublicVariables|GetM_TurretBase))
  (Rendering|Material|SetMaterial (Variables|Default|GetTurretHead) 0 (Variables|PublicVariables|GetM_TurretHead))
  (Rendering|Material|SetMaterial (Variables|Default|GetTurretBarrel) 0 (Variables|PublicVariables|GetM_TurretBarrel)))

(fn TurretRotationonTargetAI
  (bind _turretheadroot (Variables|Default|GetTurretHeadRoot))
  ;[0 0.1344 1] TargetLocking Logic
  (Transformation|SetWorldRotation (Variables|Default|GetTurretHeadRoot) (Math|Interpolation|RInterpTo (Transformation|GetWorldRotation _turretheadroot) (Math|Rotator|FindLookatRotation (Transformation|GetWorldLocation _turretheadroot) (Transformation|GetActorLocation (Variables|PrivateVariables|GetTargetAI))) 0.2 0.5) false false))

(fn ShootFunction
  ;[0 0.1344 1] Line Trace target and spawn bullet
  (Collision|LineTraceForObjects (Transformation|GetWorldLocation (Variables|Default|GetTurretBarrel)) (Transformation|GetActorLocation (Variables|PrivateVariables|GetTargetAI)) (Utilities|Array|MakeArray "ObjectTypeQuery3") false 0 "ForOneFrame")
  (bind _returnvalue (Game|SpawnActorfromClass "/Game/BluePrint/Bullet.Bullet_C" (Math|Transform|MakeTransform (+ (Transformation|GetWorldLocation (Variables|Default|GetTurretBarrel)) "0,10.000000,-10.000000") (Transformation|GetWorldRotation (Variables|Default|GetTurretHead)) "3.000000,3.000000,3.000000") "Undefined" 0 0))
  (Variables|/Game/BluePrint/Bullet.Bullet_C|SetDamageValue _returnvalue (Variables|PublicVariables|GetTurretDamageValue))
  (Default|Homing _returnvalue (Variables|/Game/BluePrint/AI.AI_C|GetCube (Variables|PrivateVariables|GetTargetAI))))