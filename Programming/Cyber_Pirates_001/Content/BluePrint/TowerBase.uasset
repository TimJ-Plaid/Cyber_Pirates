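; Tower base actor that serves as a build spot where the player spawns a GunNest, NanoBomber or RailGun turret.
; Clicking it enables input, and keys 1–3 pick the turret type once AllowInput is set.
; Hovering opens a Tick gate that turns on custom-depth highlighting and spawns the chosen turret at TowerRoot, then closes.
; Only GunNest is saved in TurretRef, and cursor exit leaves AllowInput true.
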(event OnEndCursorOver(TowerBase)
  (params (TouchedComponent :type Primitive%20Component%20Object%20Reference))
  (Variables|Default|SetAllowInput true)
  (Rendering|SetRenderCustomDepth (Variables|Default|GetTowerBase) false)
  (CallFunction|Close))

(event OnClicked(TowerBase)
  (params (TouchedComponent :type Primitive%20Component%20Object%20Reference) (ButtonPressed :type Key%20Structure :default "AnyKey"))
  (Input|EnableInput (Game|GetPlayerController 0)))

(event OnBeginCursorOver(TowerBase)
  (params (TouchedComponent :type Primitive%20Component%20Object%20Reference))
  (Utilities|FlowControl|Gate true) ; enters at Open
)

(event Custom|Close
  (Utilities|FlowControl|Gate true) ; enters at Close
)

(event EventBeginPlay)

(event Collision|EventActorBeginOverlap
  (params (OtherActor :type Actor%20Object%20Reference)))

(event EventTick
  (params (DeltaSeconds :type Float%20%28single-precision%29))
  (Utilities|FlowControl|Gate true
    (:Exit
      (Variables|Default|SetAllowInput true)
      (Rendering|SetRenderCustomDepth (Variables|Default|GetTowerBase) true)
      (if (Variables|Default|GetButtonPressed)
        (switch int (Variables|Default|GetTypeOfTurret)
          (:0
            (bind _returnvalue (Game|SpawnActorfromClass "/Game/BluePrint/GunNest.GunNest_C" (Math|Transform|MakeTransform (Transformation|GetWorldLocation (Variables|Default|GetTowerRoot))) "Undefined" 0 0))
            (Variables|Default|SetTurretRef _returnvalue))
          (:1
            (Game|SpawnActorfromClass "/Game/BluePrint/NanoBomber.NanoBomber_C" (Math|Transform|MakeTransform (Transformation|GetWorldLocation (Variables|Default|GetTowerRoot))) "Undefined" 0 0)
            (Variables|Default|SetTurretRef 0))
          (:2
            (Game|SpawnActorfromClass "/Game/BluePrint/RailGun.RailGun_C" (Math|Transform|MakeTransform (Transformation|GetWorldLocation (Variables|Default|GetTowerRoot))) "Undefined" 0 0)
            (Variables|Default|SetTurretRef 0)))
        (Variables|Default|SetButtonPressed false)
        (CallFunction|Close)))))

(event Input|KeyboardEvents|1
  (params (Key :type Key%20Structure :default "AnyKey"))
  (:Pressed
    (if (Variables|Default|GetAllowInput)
      (Variables|Default|SetButtonPressed true)
      (Variables|Default|SetTypeOfTurret 0))))

(event Input|KeyboardEvents|2
  (params (Key :type Key%20Structure :default "AnyKey"))
  (:Pressed
    (if (Variables|Default|GetAllowInput)
      (Variables|Default|SetButtonPressed true)
      (Variables|Default|SetTypeOfTurret 1))))

(event Input|KeyboardEvents|3
  (params (Key :type Key%20Structure :default "AnyKey"))
  (:Pressed
    (if (Variables|Default|GetAllowInput)
      (Variables|Default|SetButtonPressed true)
      (Variables|Default|SetTypeOfTurret 2))))

(fn ConstructionScript)