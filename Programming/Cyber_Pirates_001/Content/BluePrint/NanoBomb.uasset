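; NanoBomb is a homing projectile actor that slows AI characters it hits.
; Its Homing event hands a target component to the ProjectileMovement component and turns on homing with a high acceleration.
; When BombCollision begins overlapping an AI, the bomb sets that character's max walk speed to SlowValue, then destroys itself after a short delay.
; The file contains no logic to restore the slowed speed.
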(event OnComponentBeginOverlap(BombCollision)
  (params (OverlappedComponent :type Primitive%20Component%20Object%20Reference) (OtherActor :type Actor%20Object%20Reference) (OtherComp :type Primitive%20Component%20Object%20Reference) (OtherBodyIndex :type Integer) (bFromSweep :type Boolean) (SweepResult :type Hit%20Result%20Structure%20%28by%20ref%29))
  ;[1 1 1] When Bomb hit AI destroy Bomb
  (bind _asai (Utilities|Casting|CastToAI OtherActor))
  (Variables|/Script/Engine.CharacterMovementComponent|SetMaxWalkSpeed (Variables|/Script/Engine.Character|GetCharacterMovement _asai) (Variables|Default|GetSlowValue))
  (Utilities|FlowControl|Delay 0.2)
  (Actor|DestroyActor))

(event Custom|Homing
  (params (Target :type Static%20Mesh%20Component%20Object%20Reference))
  (bind _projectilemovement (Variables|Default|GetProjectileMovement))
  ;[1 0 0] Bullet homing event
  (Variables|/Script/Engine.ProjectileMovementComponent|SetHomingTargetComponent _projectilemovement Target)
  (Variables|/Script/Engine.ProjectileMovementComponent|SetbIsHomingProjectile _projectilemovement true)
  (Variables|/Script/Engine.ProjectileMovementComponent|SetHomingAccelerationMagnitude _projectilemovement 3.5e+04))

(fn ConstructionScript)