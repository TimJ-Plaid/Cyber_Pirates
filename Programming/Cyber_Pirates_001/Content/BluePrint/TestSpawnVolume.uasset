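; Test spawn volume that spawns AI actors at the location of its SpawnArea component.
; BeginPlay waits a few seconds, then opens a Gate that Tick feeds.
; A short Delay after the Gate throttles per-frame execution into timed spawns, each incrementing SpawnCount.
; The Gate closes once SpawnCount reaches its fixed limit.
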(event EventBeginPlay
  ;[1 0 0] When game starts spawn AI
  (Utilities|FlowControl|Delay 5.0)
  (CallFunction|SpawnAI))

(event EventTick
  (params (DeltaSeconds :type Float%20%28single-precision%29))
  ;[1 1 1] For Every Frame Spawn AI by Spawn Count
  (Utilities|FlowControl|Gate true
    (:Exit
      (Utilities|FlowControl|Delay 0.5)
      (Game|SpawnActorfromClass "/Game/BluePrint/AI.AI_C" (Math|Conversions|ToTransform(Vector) (Transformation|GetWorldLocation (Variables|Default|GetSpawnArea))) "Undefined" 0 0)
      (Variables|Default|SetSpawnCount (+ 1 (Variables|Default|GetSpawnCount)))
      (if (>= (Variables|Default|GetSpawnCount) 15)
        (CallFunction|StopSpawning)))))

(event EventSpawnAI
  ;[1 1 1] For Every Frame Spawn AI by Spawn Count
  (Utilities|FlowControl|Gate true) ; enters at Open
)

(event EventStopSpawning
  ;[1 1 1] For Every Frame Spawn AI by Spawn Count
  (Utilities|FlowControl|Gate true) ; enters at Close
)

(fn ConstructionScript)